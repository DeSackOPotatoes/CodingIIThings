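; BP_CameraDoor is a door that slides down to open while the player's view blends to the door's camera.
; OpenDoor, gated by Closed, registers the door in the game mode's LevelSave, blends the view over, plays the slide timeline, then waits and blends back to the passed view target.
; quietOpen runs the same slide without camera or save changes, and sets Closed to true when finished.
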(event `quietOpen`
  (bind (_direction _newtrack_0) (`Timeline|Timeline_0`)
    (:`Update`
      (`SceneComponent.K2_SetRelativeLocation` (`self.Door`) (`KismetMathLibrary.VLerp` (0.0 0.0 150.0) (0.0 0.0 -130.0) _newtrack_0) false false))
    (:`Finished`
      (set `self.Closed` true))))

(event `OpenDoor`
  (params (NewViewTarget :type "Actor Object Reference"))
  (if (`self.Closed`)
    (bind _asgm_coding_ii4real (cast `/Game/NEWNEWSAVES/GM_CodingII4Real` (`GameplayStatics.GetGameMode`)))
    (`KismetArrayLibrary.Array_AddUnique` (`/Game/NEWNEWSAVES/SG_LevelSave.OpenDoors` (`/Game/NEWNEWSAVES/GM_CodingII4Real.Level Save` _asgm_coding_ii4real)) self)
    (`PlayerController.SetViewTargetWithBlend` (`GameplayStatics.GetPlayerController` 0) self (`self.Blend Time`) "VTBlend_Cubic" 0.0 true)
    (`KismetSystemLibrary.Delay` (`self.Blend Time`))
    (bind (_direction _newtrack_0) (`Timeline|Timeline`)
      (:`Update`
        (`SceneComponent.K2_SetRelativeLocation` (`self.Door`) (`KismetMathLibrary.VLerp` (0.0 0.0 150.0) (0.0 0.0 -130.0) _newtrack_0) false false))
      (:`Finished`
        ;[1 1 1] Move camera back to player
        (`KismetSystemLibrary.Delay` 2.0) ; waiting 2 seconds while the door opens
        (`PlayerController.SetViewTargetWithBlend` (`GameplayStatics.GetPlayerController` 0) NewViewTarget (/ (`self.Blend Time`) 2.0) "VTBlend_Cubic" 0.0 false) ; shift camera back to player
      ))))

(fn `UserConstructionScript`)