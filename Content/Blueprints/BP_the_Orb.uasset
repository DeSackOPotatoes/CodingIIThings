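; BP_the_Orb is an orb actor that changes color and records itself as pondered when the third-person character overlaps its collision sphere.
; On overlap it gets the level save from GM_CodingII4Real, applies a dynamic material with a random Color, and adds itself uniquely to the PonderedOrb array.
; A missing save only prints an error, and the loadPonderedOrb event is an empty stub.
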(event `self.sphereCollision.OnComponentBeginOverlap`
  (params (OverlappedComponent :type "PrimitiveComponent Object Reference") (OtherActor :type "Actor Object Reference") (OtherComp :type "PrimitiveComponent Object Reference") (OtherBodyIndex :type Integer) (bFromSweep :type Boolean) (SweepResult :type "HitResult Structure (by ref)"))
  (cast `/Game/ThirdPerson/Blueprints/BP_ThirdPersonCharacter` OtherActor)
  (bind _asgm_coding_ii4real (cast `/Game/Blueprints/NEWNEWSAVES/GM_CodingII4Real` (`GameplayStatics.GetGameMode`)))
  (bind _level_save (`/Game/Blueprints/NEWNEWSAVES/GM_CodingII4Real.Level Save` _asgm_coding_ii4real))
  (`/Engine/EditorBlueprintResources/StandardMacros.IsValid` _level_save
    (:`Is Valid`
      (bind _returnvalue (`PrimitiveComponent.CreateDynamicMaterialInstance` (`self.Sphere`) 0 "/Game/Materials/theOrbColor.theOrbColor" "None"))
      (`MaterialInstanceDynamic.SetVectorParameterValue` _returnvalue "Color" (make `LinearColor` (`KismetMathLibrary.RandomFloat`) (`KismetMathLibrary.RandomFloat`) (`KismetMathLibrary.RandomFloat`) (`KismetMathLibrary.RandomFloat`)))
      (`KismetArrayLibrary.Array_AddUnique` (`/Game/Blueprints/NEWNEWSAVES/SG_LevelSave.PonderedOrb` _level_save) self))
    (:`Is Not Valid`
      (`KismetSystemLibrary.PrintString` "Orb could not find Level Save"))))

(event `loadPonderedOrb`)

(fn `UserConstructionScript`)