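; Weapon Blueprint with a type, an elemental type and a randomizable damage range, shown through its mesh, material and text labels.
; RandomizedValues raises minimum damage by a small random amount, derives the maximum from it, then refreshes text, mesh and material.
; Weapon type and element enums convert to integers that index the mesh and material arrays.
; BeginPlay and the construction script are empty, so nothing here triggers randomization.
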(event `Update Text`
  (`TextRenderComponent.K2_SetText` (`self.TextWeaponType`) (`KismetTextLibrary.Conv_StringToText` (`|GetEnumeratorNameAsString` (`self.WeaponType`))))
  (`TextRenderComponent.K2_SetText` (`self.TextElemType`) (`KismetTextLibrary.Conv_StringToText` (`|GetEnumeratorNameAsString` (`self.ElementalType`))))
  (`TextRenderComponent.K2_SetText` (`self.TextDamageValue`) (`KismetTextLibrary.Conv_StringToText` (`KismetStringLibrary.Concat_StrStr` (`KismetStringLibrary.Conv_IntToString` (`self.minDamage`)) "-" (`KismetStringLibrary.Conv_IntToString` (`self.maxDamage`))))))

(event `Randomized Values`
  (bind _output_get (set `self.minDamage` (+ (`self.minDamage`) (`KismetMathLibrary.RandomInteger` 2))))
  (set `self.maxDamage` (+ _output_get (`KismetMathLibrary.RandomIntegerInRange` 1 4)))
  (`self.Update Text`)
  (`self.setMesh`)
  (`self.setMaterial`))

(event `setMesh`
  (`StaticMeshComponent.SetStaticMesh` (`self.WeaponBody`) (`|GetArrayItem` (`self.weaponMeshes`) (`KismetMathLibrary.Conv_ByteToInt` (`self.WeaponType`)))))

(event `setMaterial`
  (`PrimitiveComponent.SetMaterial` (`self.WeaponBody`) 0 (`|GetArrayItem` (`self.materialMesh`) (`KismetMathLibrary.Conv_ByteToInt` (`self.ElementalType`)))))

(fn `UserConstructionScript`)