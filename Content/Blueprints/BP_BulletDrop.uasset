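; BP_BulletDrop is a debug actor that visualizes bullet drop from an arrow component on BeginPlay, then destroys itself after a short delay.
; A hand-rolled loop steps position by velocity, adds a frequency-derived gravity term to Z, draws lines and spheres, and line-traces each segment using the NoCollision profile, stopping on a hit.
; The engine's PredictProjectilePath then draws a path from StartingVelocity alongside it.
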(event `reallyCoolBulletDropCalculator`
  (set `self.end` (+ (`self.Start`) (/ (`self.Velocity`) (`KismetMathLibrary.MakeVector` (`self.simFrequency`) 1.0 1.0))))
  (for _ (range 1 (+ (`KismetMathLibrary.FTrunc` (`self.simFrequency`)) 1))
    (`KismetSystemLibrary.DrawDebugLine` (`self.Start`) (`self.end`) (struct :`R` 1.0 :`B` 0.789335 :`A` 1.0) (`self.maxSimTime`))
    (`KismetSystemLibrary.DrawDebugSphere` (`self.end`) 5.0 12 (struct :`R` 0.279407 :`G` 0.691337 :`B` 1.0 :`A` 1.0) (`self.maxSimTime`))
    (bind (_outhit _returnvalue) (`KismetSystemLibrary.LineTraceSingleByProfile` :`Start` (`self.Start`) :`End` (`self.end`) :`ProfileName` "NoCollision" :`DrawDebugType` "ForDuration"))
    (if _returnvalue
      (`KismetSystemLibrary.PrintString` "We hit something!")
      (break)
      (else
        (set `self.Start` (`self.end`))
        ;[1 1 1] Add Gravity to velocity
        (set `self.Velocity` (+ (`self.Velocity`) (`KismetMathLibrary.MakeVector` 0.0 0.0 (/ (`KismetMathLibrary.Square` (`self.simFrequency`)) -980.0))))
        ;[1 1 1] Set end to the  NEW start position plus velocity (where the bullet lands)
        (set `self.end` (+ (`self.Start`) (/ (`self.Velocity`) (`KismetMathLibrary.MakeVector` (`self.simFrequency`) 1.0 1.0)))))))
  (set `self.Start` (`SceneComponent.K2_GetComponentLocation` (`self.Arrow1`)))
  (set `self.Velocity` (`self.startingVelocity`)))

(event `self.ReceiveBeginPlay`
  (bind _returnvalue (`SceneComponent.K2_GetComponentLocation` (`self.Arrow1`)))
  (set `self.Start` _returnvalue)
  (`|ExecutionSequence`
    (:`then_0`
      (`self.reallyCoolBulletDropCalculator`))
    (:`then_1`
      (`GameplayStatics.Blueprint_PredictProjectilePath_Advanced` (make `PredictProjectilePathParams` _returnvalue (`self.startingVelocity`) true 0.0 (`self.maxSimTime`) true "ECC_WorldStatic" _ _ (`self.simFrequency`) 0.0 "ForDuration") :!label _label)
      (`KismetSystemLibrary.Delay` 1.5)
      (`self.K2_DestroyActor`)
      (goto _label))))

(fn `UserConstructionScript`)