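; Game mode that keeps a per-level save, using the current level name as the slot name.
; On BeginPlay it loads the SG_LevelSave to restore collected coins, open doors and player position, or creates one if none exists.
; CheckPoint saves the player transform, and FinishedLevel resets it, a zero location meaning no reposition.
; A save of another class is deleted, with no replacement created in that run.
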(event `self.ReceiveBeginPlay`
  (bind _level_save (`self.Level Save`))
  (bind _playertransform_location (`KismetMathLibrary.BreakTransform` (`/Game/Blueprints/NEWNEWSAVES/SG_LevelSave.PlayerTransform` _level_save)))
  ;[1 1 1] Is there a level save file for this level's name? If not, create one, so that we can start editing it. If there is - load it and store it to the "Level Save" variable,  so we can start editing it.
  (`KismetSystemLibrary.PrintString` "Loaiding GM_CodingII4Real" true true (struct :`R` 1.0 :`G` 0.105131 :`B` 0.035434 :`A` 1.0))
  (bind _returnvalue (`GameplayStatics.GetCurrentLevelName` true))
  (bind _returnvalue_2 (`GameplayStatics.DoesSaveGameExist` _returnvalue))
  (if _returnvalue_2
    (bind _returnvalue_3 (`GameplayStatics.LoadGameFromSlot` _returnvalue))
    (bind _assg_level_save (cast `/Game/Blueprints/NEWNEWSAVES/SG_LevelSave` _returnvalue_3)
      (:`then`
        (bind _output_get (set `self.Level Save` _assg_level_save))
        ;;[1 1 1] Change da Coins
        (`/Game/Blueprints/NEWNEWSAVES/SG_LevelSave.LoadCollectedCoins` _output_get)
        (`/Game/Blueprints/NEWNEWSAVES/SG_LevelSave.LoadOpenDoors` _output_get)
        (`KismetSystemLibrary.Delay` 0.2)
        (if (`KismetMathLibrary.EqualExactly_VectorVector` _playertransform_location)
          (`KismetSystemLibrary.PrintString` "Player location is 0")
          (else
            (`SceneComponent.K2_SetWorldTransform` (`Character.CapsuleComponent` (`GameplayStatics.GetPlayerCharacter` 0)) (`/Game/Blueprints/NEWNEWSAVES/SG_LevelSave.PlayerTransform` _level_save) false false))))
      (:`CastFailed`
        (`KismetSystemLibrary.PrintString` "Cast to SG_Level Save Failed, Deleting")
        ;[1 1 1] Delete the old save form diffrent save game types
        (`GameplayStatics.DeleteGameInSlot` _returnvalue)))
    (else
      (bind _returnvalue_4 (`GameplayStatics.CreateSaveGameObject` "/Game/Blueprints/NEWNEWSAVES/SG_LevelSave.SG_LevelSave_C"))
      (set `self.Level Save` _returnvalue_4)
      (`KismetSystemLibrary.PrintString` "Created new SG_Level Save"))))

(event `SaveGame`
  (bind _returnvalue (`GameplayStatics.GetCurrentLevelName` true))
  (`GameplayStatics.SaveGameToSlot` (`self.Level Save`) _returnvalue)
  (if true
    (`KismetSystemLibrary.PrintString` "Saved Level")
    (else
      (`KismetSystemLibrary.PrintString` "Save Level Failed"))))

(fn `CheckPoint`
  (params (`Player Transform` :type "Transform Structure"))
  (set `/Game/Blueprints/NEWNEWSAVES/SG_LevelSave.PlayerTransform` `Player Transform` (`self.Level Save`))
  (`self.SaveGame`)
  (`KismetSystemLibrary.PrintString` "Player Position Saved"))

(fn `Finished Level`
  ;[1 1 1] Reset player sart locatin to 0,0,0
  (set `/Game/Blueprints/NEWNEWSAVES/SG_LevelSave.PlayerTransform` (struct) (`self.Level Save`))
  (`self.SaveGame`))

(fn `UserConstructionScript`)