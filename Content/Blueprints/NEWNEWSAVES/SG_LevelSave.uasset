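; SG_LevelSave is a level save object that restores the state of collected coins, open doors and pondered orbs.
; Each load function loops over stored references, skipping invalid ones: coins get LoadCollectedState and doors get QuietOpen.
; LoadPonderedOrb is unfinished, with no array wired into its loop and no action on valid elements.
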(fn `LoadCollectedCoins`
  (bind _savedcollectedcoins (`self.SavedCollectedCoins`))
  (`KismetSystemLibrary.PrintString` null "Starting to load collected coins")
  (if (> (`KismetArrayLibrary.Array_Length` _savedcollectedcoins) 0)
    (for _array_element _savedcollectedcoins
      (`/Engine/EditorBlueprintResources/StandardMacros.IsValid` _array_element
        (:`Is Valid`
          (`/Game/Blueprints/BP_Coin.Load Collected State` _array_element))))))

(fn `LoadOpenDoors`
  (if true
    (for _array_element (`self.OpenDoors`)
      (`/Engine/EditorBlueprintResources/StandardMacros.IsValid` _array_element
        (:`Is Valid`
          (`/Game/Blueprints/BP_CameraDoor.quietOpen` _array_element))))))

(fn `LoadPonderedOrb`
  (`KismetSystemLibrary.PrintString` null "Pondering Orb...")
  (if (> (`KismetArrayLibrary.Array_Length` (`self.PonderedOrb`)) 0)
    (for _array_element _
      (`/Engine/EditorBlueprintResources/StandardMacros.IsValid` _array_element))))