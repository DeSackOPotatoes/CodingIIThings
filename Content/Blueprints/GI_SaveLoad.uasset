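; GI_SaveLoad, apparently a Game Instance, saves and restores player stamina, location and ability flags through an SG_Coding2 object in Slot1.
; SaveGame copies character values into an existing save and writes it; without one, it only creates the object, writing nothing.
; LoadGame applies saved values to BP_ThirdPersonCharacter, but sets CanSprint from CanShoot, leaving saved PlayerCanSprint unused.
; The Status function is empty.
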(event `SaveGame`
  (`KismetSystemLibrary.PrintString` "Starting SaveGame")
  (`GameplayStatics.DoesSaveGameExist` (`self.Slot1`))
  (if true
    (bind _returnvalue (`GameplayStatics.LoadGameFromSlot` (`self.Slot1`)))
    (bind _output_get (set `self.Saver Subclass` _returnvalue))
    ;[1 0.8763 0.3082] SaveGame Data
    (bind _assg_coding_2 (cast `/Game/Blueprints/SG_Coding2` _output_get))
    ;[1 1 1] GetPlayer INfo
    (bind _asbp_third_person_character (cast `/Game/ThirdPerson/Blueprints/BP_ThirdPersonCharacter` (`GameplayStatics.GetPlayerCharacter` 0)))
    (set `/Game/Blueprints/SG_Coding2.PlayerStamina` (`/Game/ThirdPerson/Blueprints/BP_ThirdPersonCharacter.Stamina` _asbp_third_person_character) _assg_coding_2)
    (set `/Game/Blueprints/SG_Coding2.PlayerLocation` (`Actor.K2_GetActorLocation` _asbp_third_person_character) _assg_coding_2)
    (set `/Game/Blueprints/SG_Coding2.PlayerCanSprint` (`/Game/ThirdPerson/Blueprints/BP_ThirdPersonCharacter.CanSprint` _asbp_third_person_character) _assg_coding_2)
    (set `/Game/Blueprints/SG_Coding2.PlayerCanShoot` (`/Game/ThirdPerson/Blueprints/BP_ThirdPersonCharacter.CanShoot` _asbp_third_person_character) _assg_coding_2)
    (`GameplayStatics.SaveGameToSlot` (`self.Saver Subclass`) (`self.Slot1`))
    (else
      (bind _returnvalue_2 (`GameplayStatics.CreateSaveGameObject` "/Game/Blueprints/SG_Coding2.SG_Coding2_C"))
      (set `self.Saver Subclass` _returnvalue_2))))

(event `LoadGame`
  (`KismetSystemLibrary.PrintString` "Starting LoadGame")
  (bind _returnvalue (`GameplayStatics.DoesSaveGameExist` (`self.Slot1`)))
  (if _returnvalue
    (bind _returnvalue_2 (`GameplayStatics.LoadGameFromSlot` (`self.Slot1`)))
    (bind _asbp_third_person_character (cast `/Game/ThirdPerson/Blueprints/BP_ThirdPersonCharacter` (`GameplayStatics.GetPlayerCharacter` 0)))
    (bind _assg_coding_2 (cast `/Game/Blueprints/SG_Coding2` _returnvalue_2))
    (set `self.Saver Subclass` _assg_coding_2)
    (set `/Game/ThirdPerson/Blueprints/BP_ThirdPersonCharacter.Stamina` (`/Game/Blueprints/SG_Coding2.PlayerStamina` _assg_coding_2) _asbp_third_person_character)
    (`Actor.K2_SetActorLocation` _asbp_third_person_character (`/Game/Blueprints/SG_Coding2.PlayerLocation` _assg_coding_2) false false)
    (bind _output_get (set `/Game/ThirdPerson/Blueprints/BP_ThirdPersonCharacter.CanShoot` (`/Game/Blueprints/SG_Coding2.PlayerCanShoot` _assg_coding_2) _asbp_third_person_character))
    (set `/Game/ThirdPerson/Blueprints/BP_ThirdPersonCharacter.CanSprint` _output_get _asbp_third_person_character)))

(fn `Status`)