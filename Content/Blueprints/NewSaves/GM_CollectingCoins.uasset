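; Game mode that persists per-level coin collection and player position, and restores player health, mana and stamina.
; On BeginPlay it loads or creates a level save slot named after the current level, restoring collected coins and any non-zero saved position.
; It also loads or creates a player-stats save and copies stats onto the character.
; Checkpoint stores the player transform and FinishedLevel clears it; both write only the level save.
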(event `self.ReceiveBeginPlay`
  (bind _levelcoinsave (`self.LevelCoinSave`))
  (bind _playertransform_location (`KismetMathLibrary.BreakTransform` (`/Game/Blueprints/NEWNEWSAVES/SG_LevelSave.PlayerTransform` _levelcoinsave)))
  ;[1 1 1] At the start of every level, look for a save game with that level name. If one doesn't exist, make one! Our coins will be looking to update this list when they are collected.
  (`KismetSystemLibrary.PrintString` "Starting GM CollecingCoins")
  (`|ExecutionSequence`
    (:`then_0`
      (bind _returnvalue (`GameplayStatics.GetCurrentLevelName` true))
      (bind _returnvalue_2 (`GameplayStatics.DoesSaveGameExist` _returnvalue))
      (if _returnvalue_2
        (`KismetSystemLibrary.PrintString` "Loading game from slot")
        (bind _returnvalue_3 (`GameplayStatics.LoadGameFromSlot` _returnvalue))
        (bind _assg_level_save (cast `/Game/Blueprints/NEWNEWSAVES/SG_LevelSave` _returnvalue_3)
          (:`then`
            (set `self.LevelCoinSave` _assg_level_save)
            (`/Game/Blueprints/NEWNEWSAVES/SG_LevelSave.LoadCollectedCoins` _assg_level_save)
            (if (not (`KismetMathLibrary.EqualExactly_VectorVector` _playertransform_location))
              (`SceneComponent.K2_SetWorldTransform` (`Character.CapsuleComponent` (`GameplayStatics.GetPlayerCharacter` 0)) (`/Game/Blueprints/NEWNEWSAVES/SG_LevelSave.PlayerTransform` _levelcoinsave) false false)))
          (:`CastFailed`
            (`KismetSystemLibrary.PrintString` "failed to cast to SG_levelcollectedcoins")))
        (else
          (`KismetSystemLibrary.PrintString` "creating a new save game")
          (bind _returnvalue_4 (`GameplayStatics.CreateSaveGameObject` "/Game/Blueprints/NEWNEWSAVES/SG_LevelSave.SG_LevelSave_C"))
          (set `self.LevelCoinSave` _returnvalue_4))))
    (:`then_1`
      (bind _returnvalue_5 (`GameplayStatics.DoesSaveGameExist` (`self.PlayerSaveSlotName`)))
      (if _returnvalue_5
        (bind _returnvalue_6 (`GameplayStatics.LoadGameFromSlot` (`self.PlayerSaveSlotName`)))
        (bind _assg_player_stats (cast `/Game/Blueprints/NewSaves/SG_PlayerStats` _returnvalue_6))
        (set `self.playerStatsSave` _assg_player_stats)
        (`self.Load Stats`)
        (else
          (bind _returnvalue_7 (`GameplayStatics.CreateSaveGameObject` "/Game/Blueprints/NewSaves/SG_PlayerStats.SG_PlayerStats_C"))
          (set `self.playerStatsSave` _returnvalue_7))))))

(event `Save Game`
  ;[1 1 1] When we leave a level using BP_ChangeLevel, we'll save the game.
  (bind _returnvalue (`GameplayStatics.GetCurrentLevelName` true))
  (bind _returnvalue_2 (`GameplayStatics.SaveGameToSlot` (`self.LevelCoinSave`) _returnvalue))
  (if _returnvalue_2
    (`KismetSystemLibrary.PrintString` "GameSaved!")
    (else
      (`KismetSystemLibrary.PrintString` "Game NOT saved"))))

(event `Load Stats`
  (bind _playerstatssave (`self.playerStatsSave`))
  (bind _asbp_third_person_character (cast `/Game/ThirdPerson/Blueprints/BP_ThirdPersonCharacter` (`GameplayStatics.GetPlayerCharacter` 0)))
  (set `/Game/ThirdPerson/Blueprints/BP_ThirdPersonCharacter.Health` (`/Game/Blueprints/NewSaves/SG_PlayerStats.Health` _playerstatssave) _asbp_third_person_character)
  (set `/Game/ThirdPerson/Blueprints/BP_ThirdPersonCharacter.Mana` (`/Game/Blueprints/NewSaves/SG_PlayerStats.Mana` _playerstatssave) _asbp_third_person_character)
  (set `/Game/ThirdPerson/Blueprints/BP_ThirdPersonCharacter.Stamina` (`/Game/Blueprints/NewSaves/SG_PlayerStats.Stamina` _playerstatssave) _asbp_third_person_character))

(fn `Checkpoint`
  (params (`Player Transform` :type "Transform Structure"))
  (set `/Game/Blueprints/NEWNEWSAVES/SG_LevelSave.PlayerTransform` `Player Transform` (`self.LevelCoinSave`))
  (`self.Save Game`))

(fn `FinishedLevel`
  ;[1 1 1] Reset the Player's location to wherever the player start is.
  ; They have completed the level, and should start from the beginning next time they play this level.
  (set `/Game/Blueprints/NEWNEWSAVES/SG_LevelSave.PlayerTransform` (struct) (`self.LevelCoinSave`))
  (`self.Save Game`))

(fn `UserConstructionScript`)