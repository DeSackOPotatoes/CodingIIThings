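; BP_PatrolRoute defines a spline-based patrol path, presumably for AI, that supplies world-space patrol locations.
; Each GetPatrolPointLocation call first advances PatrolIndex by Direction, then returns that spline point's location.
; Direction flips at either end for back-and-forth traversal, though the upper flip happens only once the index reaches the point count, one past the last valid index.
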(event `incrementPatrolPointIndex`
  (set `self.patrolIndex` (+ (`self.patrolIndex`) (`self.Direction`)))
  (if (>= (`self.patrolIndex`) (`SplineComponent.GetNumberOfSplinePoints` (`self.Spline`)))
    ;[1 1 1] Flip direction
    (set `self.Direction` -1)
    (elif (<= (`self.patrolIndex`) 0)
      (set `self.Direction` 1))))

(fn `getPatrolPointLocation`
  (returns (location :type "Vector Structure"))
  (`self.incrementPatrolPointIndex`)
  (return (`SplineComponent.GetLocationAtSplinePoint` (`self.Spline`) (`self.patrolIndex`) "World")))

(fn `UserConstructionScript`)